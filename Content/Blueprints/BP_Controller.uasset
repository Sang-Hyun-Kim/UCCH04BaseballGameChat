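; BP_Controller is a controller for a networked chat feature, linking the chat window UI to BP_ChatMode.
; After a short BeginPlay delay, it finds Widget_ChatWindow and binds an event to its answer-to-controller dispatcher when the remote role is set.
; Login stores the user ID and calls OnUserLogin, while outgoing messages are forwarded to BP_ChatMode.
; Incoming notices and broadcasts only print on screen, broadcasts only with authority.
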(event Custom|OnSendMsgToServer
  (params (Msg :type String) (IsServer :type Boolean))
  (bind _asbp_chat_mode (Utilities|Casting|CastToBP_ChatMode (Game|GetGameMode)))
  (Default|GotMessagefromClient _asbp_chat_mode Msg IsServer))

(event Custom|OnLoginWithID
  (params (UserId :type String))
  (Default|CallOnUserLogin UserId)
  (Variables|Default|SetUserId UserId))

(event Custom|GotBroadcast
  (params (Msg :type String))
  (if (Ability|HasAuthority)
    (Development|PrintString Msg true true "(R=0.000000,G=0.660000,B=1.000000,A=1.000000)" 1e+01)))

(event Custom|PlayerNotice
  (params (Msg :type String) (MsgSender :type Boolean))
  (if true
    (Development|PrintString Msg true true "(R=0.000000,G=0.660000,B=1.000000,A=1.000000)" 1e+01)))

(event EventBeginPlay
  (if (not (Utilities|Enum|Equal(Enum) (Class|Actor|GetRemoteRole) "ROLE_None"))
    (Utilities|FlowControl|Delay 0.5)
    (bind _foundwidgets (Widget|GetAllWidgetsOfClass "/Game/Widgets/Widget_ChatWindow.Widget_ChatWindow_C" true))
    (bind _output_get (Variables|Default|SetWidget (Utilities|Array|Get(acopy) _foundwidgets)))
    (bind _aswidget_chat_window (Utilities|Casting|CastToWidget_ChatWindow _output_get))
    (EventDispatchers|BindEventtoProcessAnswertoController _aswidget_chat_window (EventDispatchers|CreateEvent :!event Custom|OnSendMsgToServer))))

(event EventTick
  (params (DeltaSeconds :type Float%20%28single-precision%29)))

(fn ConstructionScript)