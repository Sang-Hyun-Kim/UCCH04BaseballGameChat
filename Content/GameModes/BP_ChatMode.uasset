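; Chat game mode that runs a turn-based number baseball game between a host and a client.
; Slash-prefixed messages become three-digit guesses, validated against the turn and scored as strikes, balls and outs; other messages broadcast as chat.
; A named-function timer alternates turns, which also end on each valid guess.
; Scores and attempts live in BP_MyGameState; three strikes or exhausted attempts restart the round, with announcements sent through each BP_Controller.
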(event Custom|GotMessageFromClient
  (params (Msg :type String) (IsServer :type Boolean))
  (if (Utilities|String|StartsWith Msg "/")
    (bind _isrighttry (CallFunction|ProcessNumAnswer Msg IsServer))
    (if _isrighttry
      (if (Variables|Default|GetIsFinished)
        (bind _outactors (Actor|GetAllActorsOfClass "/Script/Engine.GameStateBase"))
        (for _array_element _outactors
          (bind _asbp_my_game_state (Utilities|Casting|CastToBP_MyGameState _array_element))
          (if (Variables|Default|GetIsHostTurn)
            (Class|MyGameStateBase|ServerSetHostScore _asbp_my_game_state (+ (Variables|/Script/SampleChat.MyGameStateBase|GetHostPlayerScore _asbp_my_game_state) 1))
            (else
              (Class|MyGameStateBase|ServerSetGuestScore _asbp_my_game_state (+ (Variables|/Script/SampleChat.MyGameStateBase|GetGuestPlayerScore _asbp_my_game_state) 1))))
          ;[0.15 0.15 0.15 0.5] 게임 재시작
          (Variables|Default|SetIsHostTurn true)
          (Variables|Default|SetIsFinished false)
          (Utilities|FlowControl|Sequence
            (:then_0
              (bind _returnvalue (Class|NumBaseballBPFuncLib|RandomNumberGenerator))
              (Variables|Default|SetCurrentBBAnswer _returnvalue)
              (CallFunction|ClearAttempts)
              (bind _outactors_2 (Actor|GetAllActorsOfClass "/Script/Engine.PlayerController"))
              (for _array_element_2 _outactors_2
                (bind _asbp_controller (Utilities|Casting|CastToBP_Controller _array_element_2))
                (Default|GotBroadcast _asbp_controller "점수가 추가되었고 게임이 재시작 되었습니다.")))
            (:then_1
              (bind _scoreboardstring (CallFunction|PrintCurrentScores))
              (bind _outactors_3 (Actor|GetAllActorsOfClass "/Script/Engine.PlayerController"))
              (for _array_element_3 _outactors_3
                (bind _asbp_controller_2 (Utilities|Casting|CastToBP_Controller _array_element_3))
                (Default|GotBroadcast _asbp_controller_2 _scoreboardstring)))
            (:then_2
              (CallFunction|InitTurnTimer))))
        (else
          (CallFunction|UpdateAttempts IsServer)
          (bind _isdraw (CallFunction|CheckAttempts))
          (if _isdraw
            (Utilities|FlowControl|Sequence
              (:then_0
                (bind _outactors_4 (Actor|GetAllActorsOfClass "/Script/Engine.PlayerController"))
                (for _array_element_4 _outactors_4
                  (bind _asbp_controller_3 (Utilities|Casting|CastToBP_Controller _array_element_4))
                  (Default|GotBroadcast _asbp_controller_3 "무승부로 게임이 초기화 되었습니다.")))
              (:then_1
                ;[0.15 0.15 0.15 0.5] 게임 재시작
                (Variables|Default|SetIsHostTurn true)
                (Variables|Default|SetIsFinished false)
                (Utilities|FlowControl|Sequence
                  (:then_0
                    (bind _returnvalue_2 (Class|NumBaseballBPFuncLib|RandomNumberGenerator))
                    (Variables|Default|SetCurrentBBAnswer _returnvalue_2)
                    (CallFunction|ClearAttempts))))
              (:then_2
                (CallFunction|InitTurnTimer)))))))
    (else
      ;[0.15 0.15 0.15 0.5] 일반 채팅
      (bind _outactors_5 (Actor|GetAllActorsOfClass "/Script/Engine.PlayerController"))
      (for _array_element_5 _outactors_5
        (bind _asbp_controller_4 (Utilities|Casting|CastToBP_Controller _array_element_5))
        (Default|GotBroadcast _asbp_controller_4 Msg)))))

(event EventBeginPlay
  (bind _returnvalue (Class|NumBaseballBPFuncLib|RandomNumberGenerator))
  (Variables|Default|SetCurrentBBAnswer _returnvalue)
  (Variables|Default|SetIsHostTurn true)
  (CallFunction|InitTurnTimer))

(event EventTick
  (params (DeltaSeconds :type Float%20%28single-precision%29)))

(fn ConstructionScript)

(fn ProcessNumAnswer
  (params (NumAnsString :type String) (IsServer :type Boolean))
  (bind _ishostturn (Variables|Default|GetIsHostTurn))
  (bind _returnvalue (== IsServer _ishostturn))
  (bind _returnvalue_2 (Class|MyStringRegexValidator|ValidateBaseballInput NumAnsString))
  (bind _output_get (LocalVariables|SetCurrentValid (and _returnvalue_2 _returnvalue)))
  (if _output_get
    (Utilities|FlowControl|Sequence
      (:then_0
        (for _index (range 1 3)
          (LocalVariables|SetLocalGuessString (Utilities|String|Append (LocalVariables|GetLocalGuessString) (Utilities|Array|Get(acopy) (Utilities|String|GetCharacterArrayfromString NumAnsString) _index))))
        (bind _returnvalue_3 (Class|NumBaseballBPFuncLib|ScoreCheck (Variables|Default|GetCurrentBBAnswer) (Math|Conversions|ToInteger(Byte) (LocalVariables|GetLocalGuessString))))
        (bind _resultmessage (CallFunction|ResultCheck _returnvalue_3 (Math|Conversions|ToInteger(Byte) (LocalVariables|GetLocalGuessString))))
        (Utilities|FlowControl|Sequence
          (:then_0
            (bind _outactors (Actor|GetAllActorsOfClass "/Script/Engine.PlayerController"))
            (for _array_element _outactors
              (bind _asbp_controller (Utilities|Casting|CastToBP_Controller _array_element))
              (Default|GotBroadcast _asbp_controller _resultmessage)))
          (:then_1
            (CallFunction|OnTurnEnd))))
      (:then_1
        (return (LocalVariables|GetCurrentValid))))
    (elif _returnvalue
      (bind _outactors_2 (Actor|GetAllActorsOfClass "/Script/Engine.PlayerController"))
      (for _array_element_2 _outactors_2
        (bind _asbp_controller_2 (Utilities|Casting|CastToBP_Controller _array_element_2))
        (Default|PlayerNotice _asbp_controller_2 "입력이 유효하지 않습니다. 답안은 /와 숫자 3개의 조합으로만 해주세요" IsServer)
        (return (LocalVariables|GetCurrentValid)))
      (else
        (bind _outactors_3 (Actor|GetAllActorsOfClass "/Script/Engine.PlayerController"))
        (for _array_element_3 _outactors_3
          (bind _asbp_controller_3 (Utilities|Casting|CastToBP_Controller _array_element_3))
          (Default|PlayerNotice _asbp_controller_3 "당신의 차례가 아닙니다." IsServer)
          (return (LocalVariables|GetCurrentValid)))))))

(fn ResultCheck
  (params (Result :type Array%20of%20Integers) (Guess :type Integer))
  (LocalVariables|SetLocalResultMessage (Utilities|String|Append (Utilities|String|ToString(Integer) Guess) "에 대한 결과"))
  (if (== (Utilities|Array|Get(acopy) Result) 3)
    (Variables|Default|SetIsFinished true)
    (LocalVariables|SetLocalResultMessage (Utilities|String|Append (LocalVariables|GetLocalResultMessage) " 3 Strike로 승리하였습니다."))
    (else
      (LocalVariables|SetLocalResultMessage (Utilities|String|Append (LocalVariables|GetLocalResultMessage) " Strikes: " (Utilities|String|ToString(Integer) (Utilities|Array|Get(acopy) Result)) " Balls: " (Utilities|String|ToString(Integer) (Utilities|Array|Get(acopy) Result 1)) "Out: " (Utilities|String|ToString(Integer) (Utilities|Array|Get(acopy) Result 2))))))
  (return (LocalVariables|GetLocalResultMessage)))

(fn PrintCurrentScores
  (bind _outactors (Actor|GetAllActorsOfClass "/Script/Engine.GameStateBase"))
  (for _array_element _outactors
    (bind _asbp_my_game_state (Utilities|Casting|CastToBP_MyGameState _array_element))
    (return (Utilities|String|Append "현재 스코어 상태" "Host: " (Utilities|String|ToString(Integer) (Variables|/Script/SampleChat.MyGameStateBase|GetHostPlayerScore _asbp_my_game_state)) "점 " "Guest: " (Utilities|String|ToString(Integer) (Variables|/Script/SampleChat.MyGameStateBase|GetGuestPlayerScore _asbp_my_game_state)) "점"))))

(fn UpdateAttempts
  (params (IsServer :type Boolean))
  (bind _outactors (Actor|GetAllActorsOfClass "/Script/Engine.GameStateBase"))
  (for _array_element _outactors
    (bind _asbp_my_game_state (Utilities|Casting|CastToBP_MyGameState _array_element))
    (if IsServer
      (Class|MyGameStateBase|ServerSetHostAttemps _asbp_my_game_state (+ (Variables|/Script/SampleChat.MyGameStateBase|GetHostAttemps _asbp_my_game_state) 1))
      (else
        (Class|MyGameStateBase|ServerSetGuestAttemps _asbp_my_game_state (+ (Variables|/Script/SampleChat.MyGameStateBase|GetGuestAttemps _asbp_my_game_state) 1))))))

(fn CheckAttempts
  (bind _outactors (Actor|GetAllActorsOfClass "/Script/Engine.GameStateBase"))
  (for _array_element _outactors
    (bind _asbp_my_game_state (Utilities|Casting|CastToBP_MyGameState _array_element))
    (return (and (== (Variables|Default|GetMaxAttempt) (Variables|/Script/SampleChat.MyGameStateBase|GetHostAttemps _asbp_my_game_state)) (== (Variables|/Script/SampleChat.MyGameStateBase|GetHostAttemps _asbp_my_game_state) (Variables|/Script/SampleChat.MyGameStateBase|GetGuestAttemps _asbp_my_game_state))))))

(fn ClearAttempts
  (bind _outactors (Actor|GetAllActorsOfClass "/Script/Engine.GameStateBase"))
  (for _array_element _outactors
    (bind _asbp_my_game_state (Utilities|Casting|CastToBP_MyGameState _array_element))
    (Utilities|FlowControl|Sequence
      (:then_0
        (Class|MyGameStateBase|ServerSetGuestAttemps _asbp_my_game_state))
      (:then_1
        (Class|MyGameStateBase|ServerSetHostAttemps _asbp_my_game_state)))))

(fn InitTurnTimer
  (Utilities|Time|ClearTimerbyFunctionName 0 "OnTurnEnd")
  (bind _returnvalue (Utilities|Time|SetTimerbyFunctionName 0 "OnTurnEnd" (Variables|Default|GetTurnTime)))
  (Variables|Default|SetTurnTimerHandle _returnvalue)
  (bind _outactors (Actor|GetAllActorsOfClass "/Script/Engine.PlayerController"))
  (for _array_element _outactors
    (bind _asbp_controller (Utilities|Casting|CastToBP_Controller _array_element))
    (Default|GotBroadcast _asbp_controller "게임 시작, Host 턴이 시작되었습니다. 각 턴은 8초간 진행됩니다.")))

(fn OnTurnEnd
  (bind _turnendmessage (LocalVariables|GetTurnEndMessage))
  (Utilities|Time|ClearTimerbyFunctionName 0 "OnTurnEnd")
  (if (Variables|Default|GetIsHostTurn)
    (Variables|Default|SetIsHostTurn (not (Variables|Default|GetIsHostTurn)))
    (bind _outactors (Actor|GetAllActorsOfClass "/Script/Engine.PlayerController"))
    (for _array_element _outactors
      (bind _asbp_controller (Utilities|Casting|CastToBP_Controller _array_element))
      (Default|GotBroadcast _asbp_controller (Utilities|String|Append _turnendmessage " 이제 Client의 차례입니다."))
      (bind _returnvalue (Utilities|Time|SetTimerbyFunctionName 0 "OnTurnEnd" (Variables|Default|GetTurnTime)))
      (Variables|Default|SetTurnTimerHandle _returnvalue))
    (else
      (Variables|Default|SetIsHostTurn (not (Variables|Default|GetIsHostTurn)))
      (bind _outactors_2 (Actor|GetAllActorsOfClass "/Script/Engine.PlayerController"))
      (for _array_element_2 _outactors_2
        (bind _asbp_controller_2 (Utilities|Casting|CastToBP_Controller _array_element_2))
        (Default|GotBroadcast _asbp_controller_2 (Utilities|String|Append _turnendmessage " 이제  Host의 차례입니다."))
        (bind _returnvalue_2 (Utilities|Time|SetTimerbyFunctionName 0 "OnTurnEnd" (Variables|Default|GetTurnTime)))
        (Variables|Default|SetTurnTimerHandle _returnvalue_2)))))